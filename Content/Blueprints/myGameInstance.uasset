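; Game instance Blueprint that hosts and joins two-slot online (non-LAN) multiplayer sessions.
; HostGame creates a session and, on success, opens the third-person example map as a listen server.
; JoinGame searches for sessions, joins the first result and calls PlayerJoined, which is an empty stub.
; Failed hosting or joining prints a message, while a failed or empty search does nothing.
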(event `HostGame`
  ;[1 1 1] Host Session
  (`CreateSessionCallbackProxy.CreateSession` (`GameplayStatics.GetPlayerController` 0) 2
    (:`OnSuccess`
      (`GameplayStatics.OpenLevel` "ThirdPersonExampleMap" true "listen"))
    (:`OnFailure`
      (`KismetSystemLibrary.PrintString` "Host Failed" true true (struct :`R` 1.0 :`G` 0.007008 :`A` 1.0)))))

(event `Player Joined`)

(event `JoinGame`
  ;[1 1 1] Join Session
  (bind _results (`FindSessionsCallbackProxy.FindSessions` (`GameplayStatics.GetPlayerController` 0) 5)
    (:`OnSuccess`
      (if (> (`KismetArrayLibrary.Array_Length` _results) 0)
        (`JoinSessionCallbackProxy.JoinSession` (`GameplayStatics.GetPlayerController` 0) (`|GetArrayItem` _results)
          (:`OnSuccess`
            (`self.Player Joined`))
          (:`OnFailure`
            (`KismetSystemLibrary.PrintString` "Join failed" true true (struct :`R` 1.0 :`G` 0.007008 :`A` 1.0))))))))